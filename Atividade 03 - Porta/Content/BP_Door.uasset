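; Door actor that swings open and closed on its yaw axis through OpenDoor and CloseDoor events.
; An OpenClose timeline lerps the Door's relative yaw between closed and a right angle, playing forward to open and reversing to close.
; A Box overlap with the third-person character sets a CanOpenCloseDoor flag, though nothing in this graph reads it or triggers the door events.
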(event `OpenDoor`
  (bind (_direction _rotate_z) (`Timeline|Open/Close` :!label _label)
    (:`Update`
      (`SceneComponent.K2_SetRelativeRotation` (`self.Door`) (`KismetMathLibrary.MakeRotator` 0.0 0.0 (`KismetMathLibrary.Lerp` 0.0 90.0 _rotate_z)) false false))))

(event `CloseDoor`
  (goto _label :!via `Reverse`))

(event `self.Box.OnComponentBeginOverlap`
  (params (OverlappedComponent :type "PrimitiveComponent Object Reference") (OtherActor :type "Actor Object Reference") (OtherComp :type "PrimitiveComponent Object Reference") (OtherBodyIndex :type Integer) (bFromSweep :type Boolean) (SweepResult :type "HitResult Structure (by ref)"))
  (cast `/Game/ThirdPerson/Blueprints/BP_ThirdPersonCharacter` OtherActor)
  (set `self.CanOpen/CloseDoor?` true))

(event `self.Box.OnComponentEndOverlap`
  (params (OverlappedComponent :type "PrimitiveComponent Object Reference") (OtherActor :type "Actor Object Reference") (OtherComp :type "PrimitiveComponent Object Reference") (OtherBodyIndex :type Integer))
  (cast `/Game/ThirdPerson/Blueprints/BP_ThirdPersonCharacter` OtherActor)
  (set `self.CanOpen/CloseDoor?` false))

(fn `UserConstructionScript`)